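; Enemy pawn for a Pac-Man game that idles briefly at BeginPlay, then hunts the player.
; State changes fire a bound event that updates AI movement: Idle stops it, any other state uses MoveToActor toward the player pawn.
; When its sphere hits Pacman, it teleports Pacman to a fixed location, goes idle, and opens Level_01 after a short delay.
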(event OnComponentHit(Sphere)
  (params (HitComponent :type Primitive%20Component%20Object%20Reference) (OtherActor :type Actor%20Object%20Reference) (OtherComp :type Primitive%20Component%20Object%20Reference) (NormalImpulse :type Vector :default "0, 0, 0") (Hit :type Hit%20Result%20Structure%20%28by%20ref%29))
  (bind _aspacman_bp (Utilities|Casting|CastToPacman_BP OtherActor))
  (Transformation|SetActorLocation _aspacman_bp "1000.000000,1000.000000,1000.000000" false false)
  (Class|EnemyPawn|Idle)
  (Utilities|FlowControl|Delay 2.0)
  (Game|OpenLevel(byName) "Level_01"))

(event Custom|EventStateChangeEvent
  (EventDispatchers|BindEventtoStateChangedEvent (delegate Custom|StateChange)))

(event Custom|StateChange
  (params (NewState :type EEnemyCurrentState%20Enum :default "Default"))
  (CallFunction|UpdateMovementTarget))

(event EventBeginPlay
  (CallFunction|EventStateChangeEvent)
  (Class|EnemyPawn|Idle)
  (Utilities|FlowControl|Delay 1.5)
  (Class|EnemyPawn|Hunt))

(event Collision|EventActorBeginOverlap
  (params (OtherActor :type Actor%20Object%20Reference)))

(event EventTick
  (params (DeltaSeconds :type Float%20%28single-precision%29)))

(fn ConstructionScript)

(fn UpdateMovementTarget
  (LocalVariables|SetAIController (AI|GetAIController (Pawn|GetController)))
  (switch Utilities|FlowControl|Switch|SwitchonEEnemyCurrentState (Variables|Default|GetState)
    (:Default
      (AI|Navigation|MovetoActor (LocalVariables|GetAIController) (Game|Player|GetPlayerPawn 0) -1.0 false true true 0))
    (:Idle
      (AI|Navigation|StopMovement (LocalVariables|GetAIController)))))